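; Actor component that provides the Engineer character's abilities in the combat system.
; BeginPlay caches the owner as the Engineer third-person character.
; The first ability sets an active flag, never cleared here, and runs a Delay-based cooldown through a readiness flag.
; The second ability spawns a drone pawn ahead of the given owner, matching its rotation and assigning it as owner and instigator.
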(event `self.ReceiveBeginPlay`
  (bind _asbp_engineer_third_person_character (cast `/Game/CombatSystem/Characters/BP_EngineerThirdPersonCharacter` (`self.GetOwner`)))
  (set `self.BP_EngineerThirdPersonCharacter` _asbp_engineer_third_person_character))

(event `EngineerFirstAbility`
  ;[0.006141 1 0] First Engineer Ability
  (set `self.DoesFirstEngineerAbilityCooldownEnd` false)
  (set `self.IsFirstEngineerAbility` true)
  (`KismetSystemLibrary.Delay` 20.0)
  (set `self.DoesFirstEngineerAbilityCooldownEnd` true))

(event `SpawnDrone`
  (params (DroneOwner :type "Actor Object Reference"))
  ;[0.006141 1 0] Second Ability / Drone
  (`|SpawnActorFromClass` "/Game/CombatSystem/Drone/DronePawn.DronePawn_C" (`KismetMathLibrary.MakeTransform` (+ (* (`Actor.GetActorForwardVector` DroneOwner) 300.0) (`Actor.K2_GetActorLocation` DroneOwner)) (`Actor.K2_GetActorRotation` DroneOwner)) "AlwaysSpawn" "MultiplyWithRoot" DroneOwner DroneOwner))