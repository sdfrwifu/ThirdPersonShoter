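; Actor component implementing the sniper character's three abilities: damage over time, weapon swap and timed flight.
; The first applies looping-timer damage to a target for a set tick count.
; The swap attaches the weapon through the ShootingComponent, resetting aim, camera, ammo and walk speed while playing an equip montage.
; Movement launches the character upward into vertically steerable flight, re-asserted on Tick until it expires; it and the first ability use Delay-based cooldown flags.
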(event `self.ReceiveBeginPlay`
  (bind _asbp_sniper_third_person_character (cast `/Game/CombatSystem/Characters/BP_SniperThirdPersonCharacter` (`self.GetOwner`)))
  (set `self.BP_SniperThird PersonCharacter` _asbp_sniper_third_person_character))

(event `SniperAbilityDamageEvent`
  ;[0.006141 1 0] First Ability
  (`self.SniperAbilityDamage` (stale `SniperFirstAbility` DamagedActor)))

(event `SniperFirstAbility`
  (params (DamagedActor :type "Actor Object Reference"))
  ;[0.006141 1 0] First Ability
  (set `self.IsAbilityActive` false)
  (bind _returnvalue (`KismetSystemLibrary.K2_SetTimerDelegate` (delegate `SniperAbilityDamageEvent`) (`self.SniperAbilityTickTimeRate`) true))
  (set `self.SniperAbilityTimer` _returnvalue)
  (set `self.DoesSniperAbilityCooldownEnd` false)
  (`KismetSystemLibrary.Delay` 20.0)
  (set `self.DoesSniperAbilityCooldownEnd` true))

(event `SniperSecondAbility`
  (params (SpawnedWeapon :type "Actor Object Reference"))
  (bind _bp_sniperthird_personcharacter (`self.BP_SniperThird PersonCharacter`))
  (bind _bp_sniperthird_personcharacter_2 (`self.BP_SniperThird PersonCharacter`))
  (bind _shootingcomponent (`/Game/CombatSystem/Characters/BP_BaseThirdPersonCharacter.ShootingComponent` (`self.BP_SniperThird PersonCharacter`)))
  (bind _abp_manny (`/Game/CombatSystem/Characters/BP_BaseThirdPersonCharacter.ABP_Manny` _bp_sniperthird_personcharacter))
  (bind _shootingcomponent_2 (`/Game/CombatSystem/Characters/BP_BaseThirdPersonCharacter.ShootingComponent` (`self.BP_SniperThird PersonCharacter`)))
  ;[0.006141 1 0] Sniper Swap Weapon / Second Ability
  (`/Game/CombatSystem/Components/BP_ShootingComponent.SetDefaultFOV` _shootingcomponent)
  (set `/Game/CombatSystem/Components/BP_ShootingComponent.CanAim` false _shootingcomponent)
  (set `self.CurrentSpringArmOffset` (`SpringArmComponent.SocketOffset` (`/Game/CombatSystem/Characters/BP_BaseThirdPersonCharacter.CameraBoom` (`self.BP_SniperThird PersonCharacter`))))
  (bind _returnvalue (`KismetSystemLibrary.K2_SetTimerDelegate` (delegate `ReturnCamera`) (`self.AimingLerpTickTimeRate`) true))
  (set `self.ReturnCameraTimer` _returnvalue)
  (`/Game/CombatSystem/Components/BP_ShootingComponent.NotAimingSettings` _shootingcomponent_2)
  (`/Game/CombatSystem/Components/BP_ShootingComponent.AttachWeapon` _shootingcomponent_2 SpawnedWeapon)
  (`/Game/CombatSystem/Components/BP_ShootingComponent.SetAmmo` _shootingcomponent_2)
  (set `CharacterMovementComponent.MaxWalkSpeed` (`KismetMathLibrary.SelectFloat` (`self.MaxPistolCharacterSpeed`) (`self.MaxDefaultCharacterSpeed`) (`/Game/CombatSystem/Characters/BP_SniperThirdPersonCharacter.IsCurrentWeaponPistol` _bp_sniperthird_personcharacter_2)) (`Character.CharacterMovement` _bp_sniperthird_personcharacter_2))
  (set `/Game/Characters/Mannequins/Animations/ABP_Manny.IsUpperBody` true _abp_manny)
  (`|PlayMontage` (`Character.Mesh` _bp_sniperthird_personcharacter) "/Game/CombatSystem/Animations/AM_MM_Rifle_Equip.AM_MM_Rifle_Equip"
    (:`OnBlendOut`
      (set `/Game/Characters/Mannequins/Animations/ABP_Manny.IsUpperBody` false _abp_manny)
      (set `/Game/CombatSystem/Components/BP_ShootingComponent.CanAim` false (`/Game/CombatSystem/Characters/BP_BaseThirdPersonCharacter.ShootingComponent` _bp_sniperthird_personcharacter)))))

(event `ReturnCamera`
  ;[0.006141 1 0] Sniper Swap Weapon / Second Ability
  (`/Game/CombatSystem/Components/BP_ShootingComponent.ReturnCameraChange` (`/Game/CombatSystem/Characters/BP_BaseThirdPersonCharacter.ShootingComponent` (`self.BP_SniperThird PersonCharacter`))))

(event `LaunchCharacterUp`
  (bind _bp_sniperthird_personcharacter (`self.BP_SniperThird PersonCharacter`))
  (bind _charactermovement (`Character.CharacterMovement` _bp_sniperthird_personcharacter))
  ;[0.006141 1 0] Sniper Movement Ability
  (`|ExecutionSequence`
    (:`then_0`
      (set `self.DoesSniperMovementAbilityCooldownEnd` false)
      (`KismetSystemLibrary.Delay` 20.0)
      (set `self.DoesSniperMovementAbilityCooldownEnd` true))
    (:`then_1`
      (`Character.LaunchCharacter` _bp_sniperthird_personcharacter (0.0 0.0 1500.0) false false)
      (`CharacterMovementComponent.SetMovementMode` _charactermovement "MOVE_Flying" 0)
      (set `self.IsFlying` true)
      (`KismetSystemLibrary.Delay` 10.0)
      (set `self.IsFlying` false)
      (`CharacterMovementComponent.SetMovementMode` _charactermovement "MOVE_Falling" 0))))

(event `FlyUpDown`
  (params (ScaleValue :type "Float (double-precision)"))
  (bind _bp_sniperthird_personcharacter (`self.BP_SniperThird PersonCharacter`))
  ;[0.006141 1 0] Sniper Movement Ability
  (if (`NavMovementComponent.IsFlying` (`Character.CharacterMovement` _bp_sniperthird_personcharacter))
    (`Pawn.AddMovementInput` _bp_sniperthird_personcharacter (`Actor.GetActorUpVector` (`Pawn.GetController` _bp_sniperthird_personcharacter)) ScaleValue false)))

(event `self.ReceiveTick`
  (params (DeltaSeconds :type "Float (single-precision)"))
  ;[0.006141 1 0] Flying Mode
  (if (`self.IsFlying`)
    (`CharacterMovementComponent.SetMovementMode` (`Character.CharacterMovement` (`self.BP_SniperThird PersonCharacter`)) "MOVE_Flying" 0)))

(fn `SniperAbilityDamage`
  (params (DamagedActor :type "Actor Object Reference"))
  (locals (LocalSniperAbilityTickDamage :type "Float (double-precision)" :default 5.0) (LocalMaxAmountOfTicks :type Integer :default 4))
  (`GameplayStatics.ApplyDamage` DamagedActor (`local.LocalSniperAbilityTickDamage`))
  (bind _result (`/Engine/EditorBlueprintResources/StandardMacros.IncrementInt` (`self.AbilityAmountOfTicks`))
    (:`  `
      (if (== _result (`local.LocalMaxAmountOfTicks`))
        (set `self.AbilityAmountOfTicks` 0)
        (`KismetSystemLibrary.K2_ClearAndInvalidateTimerHandle` (`self.SniperAbilityTimer`))))))