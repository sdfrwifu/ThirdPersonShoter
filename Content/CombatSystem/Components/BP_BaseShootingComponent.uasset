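; Base weapon component for third-person shooting, handling aiming, firing, ammo HUD and montage-driven reloads.
; Looping timers drive automatic rifle and spread-shotgun fire, using camera traces to aim muzzle multi-traces or spawned normal and homing bullets.
; Trace hits apply damage, detect headshots by height and call dispatchers for ability hooks.
; Timer-stepped lerps move the camera boom for aiming and slide the weapon between idle and jog sockets, checked on Tick.
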(event `SmoothlyReAttach`
  (bind _bp_basethirdpersoncharacter (`self.BP_BaseThirdPersonCharacter`))
  (bind _righthandweaponjogsocket (`self.RightHandWeaponJogSocket`))
  (bind _righthandweaponsocket (`self.RightHandWeaponSocket`))
  (bind _currentweaponblueprint (`/Game/CombatSystem/Characters/BP_BaseThirdPersonCharacter.CurrentWeaponBlueprint` (`self.BP_BaseThirdPersonCharacter`)))
  (bind _currentweaponblueprint_2 (`/Game/CombatSystem/Characters/BP_BaseThirdPersonCharacter.CurrentWeaponBlueprint` (`self.BP_BaseThirdPersonCharacter`)))
  (bind _righthandweaponjogsocket_2 (`/Game/CombatSystem/Characters/BP_BaseThirdPersonCharacter.RightHandWeaponJogSocket` (`self.BP_BaseThirdPersonCharacter`)))
  (bind _righthandweaponsocket_2 (`/Game/CombatSystem/Characters/BP_BaseThirdPersonCharacter.RightHandWeaponSocket` (`self.BP_BaseThirdPersonCharacter`)))
  ;[0.006141 1 0 1 40] FUCKING REATTACH
  (if (not (`self.IsGrenadeThrow`))
    (set `self.IsJogging` (>= (`KismetMathLibrary.VSize` (`Actor.GetVelocity` _bp_basethirdpersoncharacter)) (`/Game/Characters/Mannequins/Animations/ABP_Manny.CharacterWalkSpeed` (`/Game/CombatSystem/Characters/BP_BaseThirdPersonCharacter.ABP_Manny` _bp_basethirdpersoncharacter))))
    (set `self.JoggingWeaponLocation` (`SceneComponent.GetSocketLocation` _righthandweaponjogsocket_2 _righthandweaponjogsocket))
    (set `self.JoggindWeaponRotation` (`SceneComponent.GetSocketRotation` _righthandweaponjogsocket_2 _righthandweaponjogsocket))
    (set `self.IdleWeaponLocation` (`SceneComponent.GetSocketLocation` _righthandweaponsocket_2 _righthandweaponsocket))
    (set `self.IdleWeaponRoatation` (`SceneComponent.GetSocketRotation` _righthandweaponsocket_2 _righthandweaponsocket))
    (if (`self.IsJogging`)
      (if (not (and (== (`Actor.K2_GetActorLocation` _currentweaponblueprint_2) (`self.JoggingWeaponLocation`)) (== (`Actor.K2_GetActorRotation` _currentweaponblueprint_2) (`self.JoggindWeaponRotation`))))
        (if (`self.IsAttachingCompleted`) :!label _label
          (set `self.IsAttachingCompleted` false)
          (bind _returnvalue (`KismetSystemLibrary.K2_SetTimerDelegate` (delegate `WeaponReAttach`) (`self.AttachLerpTickTimeRate`) true))
          (set `self.AttachTimer` _returnvalue)))
      (elif (not (and (== (`Actor.K2_GetActorRotation` _currentweaponblueprint) (`self.IdleWeaponRoatation`)) (== (`Actor.K2_GetActorLocation` _currentweaponblueprint) (`self.IdleWeaponLocation`))))
        (goto _label)))))

(event `WeaponReAttach`
  ;[0.006141 1 0 1 40] FUCKING REATTACH
  (`self.WeaponReAttachChange` (* (`self.AttachLerpChangeRate`) (`KismetMathLibrary.SelectFloat` 1.0 -1.0 (`self.IsJogging`)))))

(event `self.ReceiveBeginPlay`
  (bind _returnvalue (`self.GetOwner`))
  ;[0.006141 1 0] Begin Play Checking
  (bind _asbp_base_third_person_character (cast `/Game/CombatSystem/Characters/BP_BaseThirdPersonCharacter` (`Actor.GetOwner` _returnvalue))
    (:`then`
      ;;[0.02391 0.00239 1] У тебя на персонаже есть переменная с ABP, нет нужды здесь все это гетать -- ✓✓✓
      (set `self.BP_BaseThirdPersonCharacter` _asbp_base_third_person_character)
      (bind _asbp_base_weapon (cast `/Game/CombatSystem/Weapons/BP_BaseWeapon` _returnvalue)
        (:`then`
          (set `self.BaseWeaponBlueprint` _asbp_base_weapon)
          (bind _muzzle (`/Game/CombatSystem/Weapons/BP_BaseWeapon.Muzzle` _asbp_base_weapon))
          (`/Engine/EditorBlueprintResources/StandardMacros.IsValid` _muzzle
            (:`Is Valid`
              (`self.AttachWeapon` _asbp_base_weapon))
            (:`Is Not Valid`
              ;;[0.01293 0 1] Базовый компонент не должен содержать ссылок на персонажей, на то он и базовый  -- ✓✓✓
              (`KismetSystemLibrary.PrintString` (`KismetStringLibrary.Concat_StrStr` "Current " (`KismetSystemLibrary.GetDisplayName` _asbp_base_weapon) " doesn't have a " (`KismetSystemLibrary.GetDisplayName` _muzzle) " on the " (`KismetSystemLibrary.GetDisplayName` (`/Game/CombatSystem/Weapons/BP_BaseWeapon.WeaponMesh` _asbp_base_weapon)) ".") true true (struct :`G` 0.66 :`B` 1.0 :`A` 1.0) 10.0)
              (`self.K2_DestroyComponent`))))
        (:`CastFailed`
          (`KismetSystemLibrary.PrintString` (`KismetStringLibrary.Concat_StrStr` (`KismetSystemLibrary.GetDisplayName` self) " doesn't have an owning blueprint.") true true (struct :`G` 0.66 :`B` 1.0 :`A` 1.0) 10.0)
          (`self.K2_DestroyComponent`))))
    (:`CastFailed`
      (`KismetSystemLibrary.PrintString` (`KismetStringLibrary.Concat_StrStr` (`KismetSystemLibrary.GetDisplayName` (`self.GetOwner`)) " doesnt have an owning blueprint.") true true (struct :`G` 0.66 :`B` 1.0 :`A` 1.0) 10.0)
      (`self.K2_DestroyComponent`))))

(event `CharacterAim`
  (params (IsAiming :type Boolean))
  ;[0.006141 1 0] Character Aim
  (if (`self.CanAim`)
    (bind _output_get (set `self.IsAiming` IsAiming))
    (if _output_get
      (`self.AimingSettings`)
      (else
        (`self.NotAimingSettings`)))
    (bind _returnvalue (`KismetSystemLibrary.K2_SetTimerDelegate` (delegate `CameraLerp`) (`self.AimingLerpTickTimeRate`) true))
    (set `self.AimingTimer` _returnvalue)))

(event `self.ReceiveTick`
  (params (DeltaSeconds :type "Float (single-precision)"))
  ;[0.006141 1 0] Attach Weapon
  (`self.SmoothlyReAttach`)
  (bind _returnvalue (`|GetDataTableRow` "/Game/CombatSystem/DataTables/DT_CharacterClassStats.DT_CharacterClassStats" (`KismetStringLibrary.Conv_StringToName` (`KismetSystemLibrary.GetClassDisplayName` (`GameplayStatics.GetObjectClass` self))))))

(event `CameraLerp`
  ;[0.006141 1 0] Character Aim
  (`self.AimCameraChange` (* (`self.AimingLerpChangeRate`) (`KismetMathLibrary.SelectFloat` 1.0 -1.0 (`self.IsAiming`)))))

(event `WeaponReload`
  (params (PlayRate :type "Float (double-precision)" :default 1.0))
  (bind _montagesectionname (`self.MontageSectionName`))
  (bind _defaultclipamount (`/Game/CombatSystem/Weapons/BP_BaseWeapon.GetWeaponStats` (`self.BaseWeaponBlueprint`)))
  ;[0.006141 1 0] Weapon Reload
  (`self.OnWeaponBeginReload`)
  (if (and (`self.IsReloadCompleted`) (not (>= (`self.CurrentAmountOfAmmo`) _defaultclipamount)) (not (`AnimInstance.IsAnyMontagePlaying` (`SkeletalMeshComponent.GetAnimInstance` (`Character.Mesh` (`self.BP_BaseThirdPersonCharacter`))))))
    (set `self.IsReloadCompleted` false)
    (set `/Game/Characters/Mannequins/Animations/ABP_Manny.IsUpperBody` true (`/Game/CombatSystem/Characters/BP_BaseThirdPersonCharacter.ABP_Manny` (`self.BP_BaseThirdPersonCharacter`)))
    (if (`self.IsClipInserted`)
      (if (> (`self.CurrentAmountOfAmmo`) 0.0)
        (set `self.MontageSectionName` "NoClipNoShutter")
        (else
          (set `self.MontageSectionName` "NoClip")))
      (set `self.ReloadMontage` "/Game/CombatSystem/Animations/MM_Rifle_Reload_Montage.MM_Rifle_Reload_Montage")
      (elif (> (`self.CurrentAmountOfAmmo`) 0.0)
        (set `self.MontageSectionName` "NoShutter")
        (set `self.ReloadMontage` "/Game/CombatSystem/Animations/MM_Rifle_Reload_Montage1.MM_Rifle_Reload_Montage1")
        (else
          (set `self.MontageSectionName` "Default")
          (set `self.ReloadMontage` "/Game/CombatSystem/Animations/MM_Rifle_Reload_Montage.MM_Rifle_Reload_Montage"))))
    (`|PlayMontage` (`Character.Mesh` (`self.BP_BaseThirdPersonCharacter`)) (`self.ReloadMontage`) PlayRate 0.0 (`self.MontageSectionName`)
      (:`OnBlendOut`
        (`self.OnWeaponAddAmmo`)
        (bind _output_get (set `self.CurrentAmountOfAmmo` (+ (`self.AmmoToAdd`) _defaultclipamount)))
        (if (or (== _montagesectionname "NoShutter") (== _montagesectionname "NoClipNoShutter"))
          (`/Engine/EditorBlueprintResources/StandardMacros.IncrementFloat` _output_get
            (:`  `
              _)))
        (set `self.IsReloadCompleted` true)
        (set `/Game/Characters/Mannequins/Animations/ABP_Manny.IsUpperBody` false (`/Game/CombatSystem/Characters/BP_BaseThirdPersonCharacter.ABP_Manny` (`self.BP_BaseThirdPersonCharacter`)))
        (set `self.IsClipInserted` false)
        (`self.SetTextToWidget`))
      (:`OnInterrupted`
        (set `self.IsReloadCompleted` true)
        (set `/Game/Characters/Mannequins/Animations/ABP_Manny.IsUpperBody` false (`/Game/CombatSystem/Characters/BP_BaseThirdPersonCharacter.ABP_Manny` (`self.BP_BaseThirdPersonCharacter`)))))))

(event `Projectile`
  (params (InputAction :type "InputAction Object Reference"))
  (bind _bp_basethirdpersoncharacter (`self.BP_BaseThirdPersonCharacter`))
  (bind _returnvalue (`SceneComponent.K2_GetComponentLocation` (`/Game/CombatSystem/Weapons/BP_BaseWeapon.Muzzle` (`self.BaseWeaponBlueprint`))))
  ;[0.006141 1 0] Projectile Shooting
  (if (> (`self.CurrentAmountOfAmmo`) 0.0)
    (bind _output_get (set `self.CurrentInputAction` InputAction))
    (if (== _output_get (`self.ProjectileInputAction`))
      (set `self.ProjectileClass` "/Game/CombatSystem/Weapons/BP_Bullet.BP_Bullet_C")
      (else
        (set `self.ProjectileClass` "/Game/CombatSystem/Weapons/BP_AutoHomingBullet.BP_AutoHomingBullet_C")))
    (bind _outhit (`self.GetCameraForwardTraceHit`))
    (bind _returnvalue_2 (`|SpawnActorFromClass` (`self.ProjectileClass`) (`KismetMathLibrary.MakeTransform` _returnvalue (`KismetMathLibrary.Conv_VectorToRotator` (`KismetMathLibrary.GetDirectionUnitVector` _returnvalue (`.Location` (`GameplayStatics.BreakHitResult` _outhit))))) "AlwaysSpawn" "MultiplyWithRoot" _bp_basethirdpersoncharacter _bp_basethirdpersoncharacter))
    (`self.AmmoSubtract`)
    (set `self.CurrentBulletBlueprint` _returnvalue_2)
    (`/Game/CombatSystem/Weapons/BP_BaseWeapon.SpawnSoundAndFX` (`self.BaseWeaponBlueprint`))
    (if (not (== (`self.CurrentInputAction`) (`self.ProjectileInputAction`)))
      (`/Game/CombatSystem/Weapons/BP_AutoHomingBullet.HomingProjectile` (cast `/Game/CombatSystem/Weapons/BP_AutoHomingBullet` (`self.CurrentBulletBlueprint`) :!pure true)))))

(event `FireWeapon`
  (params (InputValue :type Boolean))
  ;[0.006141 1 0] Weapon Fire
  (if (and (`self.IsReloadCompleted`) (not (`KismetSystemLibrary.K2_IsTimerActiveHandle` (`self.FullAutoTimer`))))
    (`self.MultiTraceFire` InputValue)
    (bind _returnvalue (`KismetSystemLibrary.K2_SetTimerDelegate` (delegate `TimerEventMultiTrace`) (`.DefaultFireRate` (`/Game/CombatSystem/Weapons/BP_BaseWeapon.GetWeaponStats` (`self.BaseWeaponBlueprint`))) true))
    (set `self.FullAutoTimer` _returnvalue)))

(event `TimerEventMultiTrace`
  ;[0.006141 1 0] Weapon Fire
  (`self.MultiTraceFire` (stale `FireWeapon` InputValue)))

(event `ShotgunFireWeapon`
  (params (InputValue :type Boolean))
  ;[0.006141 1 0] Weapon Fire
  (if (and (`self.IsReloadCompleted`) (not (`KismetSystemLibrary.K2_IsTimerActiveHandle` (`self.FullAutoTimer`))))
    (`self.ShotgunMultiTraceFire` InputValue)
    (bind _returnvalue (`KismetSystemLibrary.K2_SetTimerDelegate` (delegate `EventMultiTraceFire`) (`.DefaultFireRate` (`/Game/CombatSystem/Weapons/BP_BaseWeapon.GetWeaponStats` (`self.BaseWeaponBlueprint`))) true))
    (set `self.FullAutoTimer` _returnvalue)))

(event `EventMultiTraceFire`
  ;[0.006141 1 0] Weapon Fire
  (`self.ShotgunMultiTraceFire` (stale `ShotgunFireWeapon` InputValue)))

(fn `AimCameraChange`
  (params (AimingLerpChangeRate :type "Float (double-precision)"))
  (locals (LocalLerpEndAlpha :type "Float (double-precision)" :default 1.0) (LocalLerpEndAlphaNotAiming :type "Float (double-precision)") (LocalAimingSpringArmOffset :type "Vector Structure" :default (270.0 80.0 70.0)) (LocalDefaultSpringArmOffset :type "Vector Structure"))
  (bind _aimingalpha (`self.AimingAlpha`))
  (bind _output_get (set `self.AimingAlpha` (`KismetMathLibrary.FClamp` (+ (`self.AimingAlpha`) AimingLerpChangeRate))))
  (set `SpringArmComponent.SocketOffset` (`KismetMathLibrary.VLerp` (`local.LocalDefaultSpringArmOffset`) (`local.LocalAimingSpringArmOffset`) (`KismetMathLibrary.FClamp` _output_get)) (`/Game/CombatSystem/Characters/BP_BaseThirdPersonCharacter.CameraBoom` (`self.BP_BaseThirdPersonCharacter`)))
  (if (>= _aimingalpha (`local.LocalLerpEndAlpha`))
    (`KismetSystemLibrary.K2_ClearAndInvalidateTimerHandle` (`self.AimingTimer`) :!label _label)
    (elif (<= _aimingalpha (`local.LocalLerpEndAlphaNotAiming`))
      (goto _label))))

(fn `AimingSettings`
  (locals (LocalMaxAimingCharacterSpeed :type "Float (double-precision)" :default 120.0))
  (bind _hud (`/Game/CombatSystem/Characters/BP_BaseThirdPersonCharacter.HUD` (`self.BP_BaseThirdPersonCharacter`)))
  (bind _charactermovement (`Character.CharacterMovement` (`self.BP_BaseThirdPersonCharacter`)))
  (set `CharacterMovementComponent.MaxWalkSpeed` (`local.LocalMaxAimingCharacterSpeed`) _charactermovement)
  (set `CharacterMovementComponent.bOrientRotationToMovement` false _charactermovement)
  (set `CharacterMovementComponent.bUseControllerDesiredRotation` true _charactermovement)
  (`Widget.SetVisibility` _hud "Visible")
  (`Widget.SetVisibility` (`/Game/CombatSystem/Hud/CharacterHud.ScopeImage` _hud) "Hidden")
  (`Widget.SetVisibility` (`/Game/CombatSystem/Hud/CharacterHud.AimImage` _hud) "Visible")
  (`self.OnAimingSetFOV`))

(fn `AmmoSubtract`
  (locals (LocalPlayRate :type "Float (double-precision)" :default 1.0))
  (bind _result (`/Engine/EditorBlueprintResources/StandardMacros.IncrementFloat` (`/Game/CombatSystem/Weapons/BP_BaseWeapon.GetWeaponStats` (`self.BaseWeaponBlueprint`)))
    (:`  `
      (bind _output_get (set `self.CurrentAmountOfAmmo` (`KismetMathLibrary.FClamp` (`self.CurrentAmountOfAmmo`) 0.0 _result)))
      (bind _result_2 (`/Engine/EditorBlueprintResources/StandardMacros.DecrementFloat` _output_get)
        (:`  `
          (`self.SetTextToWidget`)
          (if (== _result_2 0.0)
            (`self.WeaponReload` (`local.LocalPlayRate`))))))))

(fn `AttachSecondWeapon`
  (params (WeaponToAttach :type "Actor Object Reference"))
  (locals (LocalBackWeaponSocket :type Name :default "BackWeaponSocket"))
  (`Actor.K2_AttachToComponent` WeaponToAttach (`Character.Mesh` (`self.BP_BaseThirdPersonCharacter`)) (`local.LocalBackWeaponSocket`) "SnapToTarget" "SnapToTarget" "SnapToTarget" true))

(fn `AttachWeapon`
  (params (Weapon :type "Actor Object Reference"))
  (`Actor.K2_AttachToComponent` Weapon (`Character.Mesh` (`self.BP_BaseThirdPersonCharacter`)) (`self.RightHandWeaponSocket`) "SnapToTarget" "SnapToTarget" "SnapToTarget" true))

(fn `GetCameraForwardTraceHit`
  (returns (OutHit :type "HitResult Structure"))
  (bind _returnvalue (`GameplayStatics.GetPlayerCameraManager` 0))
  (bind _returnvalue_2 (`Actor.K2_GetActorLocation` _returnvalue))
  (bind _outhit (`KismetSystemLibrary.LineTraceSingle` :`Start` _returnvalue_2 :`End` (+ _returnvalue_2 (* (`Actor.GetActorForwardVector` _returnvalue) (`self.ShootingDistanceMultiplayer`))) :`TraceChannel` "TraceTypeQuery2" :`TraceColor` (struct :`R` 1.0 :`B` 0.826939 :`A` 1.0)))
  (return _outhit))

(fn `GetDataTableInfo`
  (returns (`Out Row` :type "/Game/CombatSystem/Structures/S_CharacterClassStats_Old Structure"))
  (bind _returnvalue (`|GetDataTableRow` "/Game/CombatSystem/DataTables/DT_CharacterClassesStats_Old.DT_CharacterClassesStats_Old" (`KismetStringLibrary.Conv_StringToName` (`KismetSystemLibrary.GetClassDisplayName` (`GameplayStatics.GetObjectClass` (`self.BP_BaseThirdPersonCharacter`)))))
    (:`then`
      (return _returnvalue))))

(fn `MultiTraceFire`
  (params (IsFiring :type Boolean))
  (locals (LocalMaxAmountOfShotsAbility :type Integer :default 5) (LocalMinLineTraceSpread :type "Float (double-precision)" :default -750.0) (LocalMaxLineTraceSpread :type "Float (double-precision)" :default 750.0) (LocalAbilitySpreadMultiplier :type "Float (double-precision)" :default 0.5))
  (bind _returnvalue (`SceneComponent.K2_GetComponentLocation` (`/Game/CombatSystem/Weapons/BP_BaseWeapon.Muzzle` (`self.BaseWeaponBlueprint`))))
  ;[0.03253 0 1] Убираем в функцию тк реюзаем
  (if (and IsFiring (> (`self.CurrentAmountOfAmmo`) 0.0) (`self.IsAiming`) (`self.IsReloadCompleted`))
    (`/Game/CombatSystem/Weapons/BP_BaseWeapon.SpawnSoundAndFX` (`self.BaseWeaponBlueprint`))
    (`self.AmmoSubtract`)
    (bind _outhit (`self.GetCameraForwardTraceHit`))
    (bind (_bblockinghit _binitialoverlap _time _distance _location _impactpoint _normal _impactnormal _physmat _hitactor _hitcomponent _hitbonename _bonename _hititem _elementindex _faceindex _tracestart _traceend) (`GameplayStatics.BreakHitResult` _outhit))
    (bind _returnvalue_2 (- _location _returnvalue))
    (bind _outhits (`KismetSystemLibrary.LineTraceMulti` :`Start` _returnvalue :`End` (`KismetMathLibrary.SelectVector` (+ (* (/ _returnvalue_2 (`KismetMathLibrary.VSize` _returnvalue_2)) (`self.ShootingDistanceMultiplayer`)) _location) _traceend _bblockinghit) :`TraceChannel` "TraceTypeQuery1" :`DrawDebugType` "ForDuration" :`bIgnoreSelf` false))
    (`self.TraceDamage` _outhits)
    (else
      (`KismetSystemLibrary.K2_ClearAndInvalidateTimerHandle` (`self.FullAutoTimer`)))))

(fn `NotAimingSettings`
  (bind _currentmaxcharacterspeed (`self.CurrentMaxCharacterSpeed`))
  (bind _bp_basethirdpersoncharacter (`self.BP_BaseThirdPersonCharacter`))
  (bind _charactermovement (`Character.CharacterMovement` (`self.BP_BaseThirdPersonCharacter`)))
  (`self.OnNotAimingSettings`)
  (set `CharacterMovementComponent.MaxWalkSpeed` (`KismetMathLibrary.SelectFloat` _currentmaxcharacterspeed (`self.MaxDefaultCharacterSpeed`) (> _currentmaxcharacterspeed 0.0)) _charactermovement)
  (set `CharacterMovementComponent.bOrientRotationToMovement` true _charactermovement)
  (set `CharacterMovementComponent.bUseControllerDesiredRotation` false _charactermovement)
  (`Widget.SetVisibility` (`/Game/CombatSystem/Characters/BP_BaseThirdPersonCharacter.HUD` (`self.BP_BaseThirdPersonCharacter`)) "Hidden")
  (`CameraComponent.SetFieldOfView` (`/Game/CombatSystem/Characters/BP_BaseThirdPersonCharacter.ThirdPersonCamera` _bp_basethirdpersoncharacter) (`/Game/CombatSystem/Characters/BP_BaseThirdPersonCharacter.DefaultFOV` _bp_basethirdpersoncharacter)))

(fn `SetAmmo`
  ;[1 1 1] Comment
  (set `self.CurrentAmountOfAmmo` (`/Game/CombatSystem/Weapons/BP_BaseWeapon.GetWeaponStats` (`/Game/CombatSystem/Characters/BP_BaseThirdPersonCharacter.CurrentWeaponBlueprint` (`self.BP_BaseThirdPersonCharacter`))))
  (`self.SetTextToWidget`))

(fn `SetTextToWidget`
  (bind _hud (`/Game/CombatSystem/Characters/BP_BaseThirdPersonCharacter.HUD` (`self.BP_BaseThirdPersonCharacter`))
    (:`then`
      (`TextBlock.SetText` (`/Game/CombatSystem/Hud/CharacterHud.AmmoAmount` _hud) (`KismetTextLibrary.Conv_DoubleToText` (`self.CurrentAmountOfAmmo`) "HalfToEven")))
    (:`else`)))

(fn `ShotgunMultiTraceFire`
  (params (IsFiring :type Boolean))
  (locals (LocalMaxAmountOfShotsAbility :type Integer :default 5) (LocalMinLineTraceSpread :type "Float (double-precision)" :default -750.0) (LocalMaxLineTraceSpread :type "Float (double-precision)" :default 750.0) (DefaultValue :type "Float (double-precision)" :default 1.0))
  (bind _engineerspreadmultiplier (`self.EngineerSpreadMultiplier`))
  (bind _localminlinetracespread (`local.LocalMinLineTraceSpread`))
  (bind _localmaxlinetracespread (`local.LocalMaxLineTraceSpread`))
  (bind _returnvalue (`SceneComponent.K2_GetComponentLocation` (`/Game/CombatSystem/Weapons/BP_BaseWeapon.Muzzle` (`self.BaseWeaponBlueprint`))))
  ;[0.03253 0 1] Убираем в функцию тк реюзаем
  (if (and IsFiring (> (`self.CurrentAmountOfAmmo`) 0.0) (`self.IsAiming`) (`self.IsReloadCompleted`))
    (`/Game/CombatSystem/Weapons/BP_BaseWeapon.SpawnSoundAndFX` (`self.BaseWeaponBlueprint`))
    (`self.AmmoSubtract`)
    (bind _outhit (`self.GetCameraForwardTraceHit`))
    (`self.OnShotgunFire`)
    (for _ (range (+ (`self.EnginnerBlastAmount`) 1))
      (bind (_bblockinghit _binitialoverlap _time _distance _location _impactpoint _normal _impactnormal _physmat _hitactor _hitcomponent _hitbonename _bonename _hititem _elementindex _faceindex _tracestart _traceend) (`GameplayStatics.BreakHitResult` _outhit))
      (bind _returnvalue_2 (- _location _returnvalue))
      (bind _outhits (`KismetSystemLibrary.LineTraceMulti` :`Start` _returnvalue :`End` (+ (`KismetMathLibrary.SelectVector` (+ (* (/ _returnvalue_2 (`KismetMathLibrary.VSize` _returnvalue_2)) (`self.ShootingDistanceMultiplayer`)) _location) _traceend _bblockinghit) (`KismetMathLibrary.MakeVector` (* (`KismetMathLibrary.RandomFloatInRange` _localminlinetracespread _localmaxlinetracespread) _engineerspreadmultiplier) (* (`KismetMathLibrary.RandomFloatInRange` _localminlinetracespread _localmaxlinetracespread) _engineerspreadmultiplier) (* (`KismetMathLibrary.RandomFloatInRange` _localminlinetracespread _localmaxlinetracespread) _engineerspreadmultiplier))) :`TraceChannel` "TraceTypeQuery1" :`DrawDebugType` "ForDuration" :`bIgnoreSelf` false))
      (`self.TraceDamage` _outhits))
    (`self.OnBlastLoopCompleted`)
    (set `self.EngineerSpreadMultiplier` (`local.DefaultValue`))
    (else
      (`KismetSystemLibrary.K2_ClearAndInvalidateTimerHandle` (`self.FullAutoTimer`)))))

(fn `TraceDamage`
  (params (OutHits :type "Array of HitResult Structure"))
  (locals (LocalIsActorDamaged :type Boolean) (LocalLastHitActor :type "Actor Object Reference") (LocalDefaultMultiplierValue :type "Float (double-precision)" :default 1.0) (LocalBottomCharacterSocketName :type Name :default "bottom_Socket"))
  (set `local.LocalIsActorDamaged` false)
  (for _array_element OutHits
    (bind (_bblockinghit _binitialoverlap _time _distance _location _impactpoint _normal _impactnormal _physmat _hitactor _hitcomponent) (`GameplayStatics.BreakHitResult` _array_element))
    (bind _asbp_base_third_person_character (cast `/Game/CombatSystem/Characters/BP_BaseThirdPersonCharacter` _hitactor)
      (:`then`
        (bind _output_get (set `/Game/CombatSystem/Characters/BP_BaseThirdPersonCharacter.HitLocation` _location _asbp_base_third_person_character))
        (if (and (!= (`local.LocalLastHitActor`) _hitactor) (not (`/Game/CombatSystem/Characters/BP_BaseThirdPersonCharacter.IsDead` _asbp_base_third_person_character)))
          (if (`KismetMathLibrary.InRange_FloatFloat` (.z (- _output_get (`SceneComponent.GetSocketLocation` _hitcomponent (`local.LocalBottomCharacterSocketName`)))) 150.0 180.0)
            (`self.OnHeadHit`))
          (`GameplayStatics.ApplyDamage` _hitactor (* (`.DefaultDamage` (`/Game/CombatSystem/Weapons/BP_BaseWeapon.GetWeaponStats` (`self.BaseWeaponBlueprint`))) (`self.DamageMultiplier`)))
          (set `self.DamageMultiplier` (`local.LocalDefaultMultiplierValue`))
          (`self.OnFirstSniperAbility` _hitactor)
          (`self.OnAddHitsInRowAmmo`)
          (set `local.LocalIsActorDamaged` true)
          (set `local.LocalLastHitActor` _hitactor)))
      (:`CastFailed`
        (if (`local.LocalIsActorDamaged`)
          _)))))

(fn `WeaponReAttachChange`
  (params (AttachLerpChangeRate :type "Float (double-precision)"))
  (locals (LocalAttachLerpEnd :type "Float (double-precision)" :default 1.0) (LocalAttachLerpEndWalk :type "Float (double-precision)" :default 0.0) (LocalMinAlphaValue :type "Float (double-precision)" :default 0.0) (LocalMaxAlphaValue :type "Float (double-precision)" :default 1.0))
  (bind _output_get (set `self.AttachAlpha` (+ (`KismetMathLibrary.FClamp` (`self.AttachAlpha`) (`local.LocalMinAlphaValue`) (`local.LocalMaxAlphaValue`)) AttachLerpChangeRate)))
  (`Actor.K2_SetActorLocationAndRotation` (`/Game/CombatSystem/Characters/BP_BaseThirdPersonCharacter.CurrentWeaponBlueprint` (`self.BP_BaseThirdPersonCharacter`)) (`KismetMathLibrary.VLerp` (`self.IdleWeaponLocation`) (`self.JoggingWeaponLocation`) _output_get) (`KismetMathLibrary.RLerp` (`self.IdleWeaponRoatation`) (`self.JoggindWeaponRotation`) _output_get true) false false)
  (if (>= (`self.AttachAlpha`) (`local.LocalAttachLerpEnd`))
    (set `self.IsAttachingCompleted` true :!label _label)
    (`KismetSystemLibrary.K2_ClearAndInvalidateTimerHandle` (`self.AttachTimer`))
    (elif (<= (`self.AttachAlpha`) (`local.LocalAttachLerpEndWalk`))
      (goto _label))))