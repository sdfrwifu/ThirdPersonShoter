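; Base weapon Blueprint that provides stat lookup, muzzle effects and ammo setup for the combat system.
; GetWeaponStats reads clip amount, fire rate and damage from DT_WeaponClassStats, using the class display name as the row name.
; BeginPlay waits one tick before calling SetAmmo on the ShootingComponent, and SpawnSoundAndFX plays the fire emitter and sound at the Muzzle.
; Tick only prints a leftover debug string.
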(event `self.ReceiveBeginPlay`
  (`KismetSystemLibrary.DelayUntilNextTick`)
  (`/Game/CombatSystem/Components/BP_BaseShootingComponent.SetAmmo` (`self.ShootingComponent`)))

(event `self.ReceiveTick`
  (params (DeltaSeconds :type "Float (single-precision)"))
  (`KismetSystemLibrary.PrintString` (`KismetStringLibrary.Conv_DoubleToString` 0.0) true true (struct :`G` 0.66 :`B` 1.0 :`A` 1.0) 2.0 "Nollllne"))

(fn `GetWeaponStats`
  (returns (DefaultClipAmount :type "Float (double-precision)") (DefaultFireRate :type "Float (double-precision)") (DefaultDamage :type "Float (double-precision)"))
  (bind _returnvalue (`|GetDataTableRow` "/Game/CombatSystem/DataTables/DT_WeaponClassStats.DT_WeaponClassStats" (`KismetStringLibrary.Conv_StringToName` (`KismetSystemLibrary.GetClassDisplayName` (`GameplayStatics.GetObjectClass` self))))
    (:`then`
      (return (`.ClipAmount_4_872091BF46B69179EF1BE89B0D4392D3` (break `/Game/CombatSystem/Structures/S_WeaponClassStats` _returnvalue)) (`.FireRate_6_52664A084E40635F073764AD889A9917` (break `/Game/CombatSystem/Structures/S_WeaponClassStats` _returnvalue)) (`.Damage_8_B282817843B7956B706AB79119A1B644` (break `/Game/CombatSystem/Structures/S_WeaponClassStats` _returnvalue))))))

(fn `SpawnSoundAndFX`
  (bind _muzzle (`self.Muzzle`))
  (bind _returnvalue (`SceneComponent.K2_GetComponentLocation` _muzzle))
  ;[0.006141 1 0] Comment
  (`GameplayStatics.SpawnEmitterAtLocation` (`self.FireEmitter`) _returnvalue (`SceneComponent.K2_GetComponentRotation` _muzzle))
  (`GameplayStatics.SpawnSoundAtLocation` (`self.FireSound`) _returnvalue (struct) 1.0 1.0 0.0 null null))

(fn `UserConstructionScript`)